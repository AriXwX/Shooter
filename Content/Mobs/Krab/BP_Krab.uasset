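; BP_Krab is an enemy crab that chases a nearby first-person player, deals contact damage and steals a random rune from the active slot.
; Once it has touched the player, it stops chasing, moves by an offset from the player's forward vector and carries any stolen rune.
; Bomb and bullet hits on two boxes deal doubled gun damage, tinting its rune plane.
; Death drops its random rune, the stolen one and BP_Mask.
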(event `self.ReceiveActorBeginOverlap`
  (params (OtherActor :type "Actor Object Reference"))
  (bind (_returnvalue_x _returnvalue_y _returnvalue_z) (`KismetMathLibrary.BreakVector` (`SceneComponent.K2_GetComponentLocation` (`self.Sphere`))))
  (bind _returnvalue (- (`KismetArrayLibrary.Array_Length` (`self.Runes`)) 1))
  (bind _output (`|GetArrayItem` (`self.Runes`) (`KismetMathLibrary.RandomIntegerInRange` 0 _returnvalue)))
  (bind (_brush_imagesize _brush_margin _brush_tintcolor _brush_resourceobject) (break `SlateBrush` (`Image.Brush` (`/Game/Runes/WBP_Slot2.Image` _output))))
  (if (not (<= (`self.Health`) 0.0))
    (bind _asfirst_person_character (cast `/Game/FirstPersonBP/FirstPersonCharacter` OtherActor))
    (set `self.HaveRune` true)
    (`GameplayStatics.ApplyDamage` _asfirst_person_character 5.0)
    (`/Engine/EditorBlueprintResources/StandardMacros.DoOnce` false
      (:`Completed`
        (bind _wbpas (`/Game/FirstPersonBP/FirstPersonCharacter.WBPAS` _asfirst_person_character))
        (for _array_element (`PanelWidget.GetAllChildren` (select `int` (`/Game/FirstPersonBP/FirstPersonCharacter.ActiveSlotNumber` _asfirst_person_character) :`0` (`/Game/Runes/ActiveSlots/WBP_ActiveSlot1.Overlay_112` (`/Game/Runes/ActiveSlots/WBP_ActiveSlots.WBP_ActiveSlot1` _wbpas)) :`1` (`/Game/Runes/ActiveSlots/WBP_ActiveSlot2.Overlay_112` (`/Game/Runes/ActiveSlots/WBP_ActiveSlots.WBP_ActiveSlot2` _wbpas)) :`2` (`/Game/Runes/ActiveSlots/WBP_ActiveSlot3.Overlay_112` (`/Game/Runes/ActiveSlots/WBP_ActiveSlots.WBP_ActiveSlot3` _wbpas))))
          (bind _aswbp_slot_2 (cast `/Game/Runes/WBP_Slot2` _array_element))
          (`KismetArrayLibrary.Array_Add` (`self.Runes`) _aswbp_slot_2))
        (if (>= _returnvalue 0)
          (bind _astexture (cast `Texture` _brush_resourceobject))
          (bind _returnvalue_2 (`|SpawnActorFromClass` (select `int` (`KismetArrayLibrary.Array_Find` (`self.ArrayTextures`) _astexture) :`0` "/Game/Runes/Loot/Damage.Damage_C" :`1` "/Game/Runes/Loot/Gravity.Gravity_C" :`2` "/Game/Runes/Loot/Radius.Radius_C" :`3` "/Game/Runes/Loot/Energy.Energy_C" :`4` "/Game/Runes/Loot/Speed.Speed_C" :`5` "/Game/Runes/Loot/ShieldDamage.ShieldDamage_C" :`6` "/Game/Runes/Loot/ShieldRegen.ShieldRegen_C" :!type "Actor Class Reference") (`KismetMathLibrary.MakeTransform` (`KismetMathLibrary.MakeVector` _returnvalue_x _returnvalue_y _returnvalue_z)) "Undefined" "OverrideRootScale" null null))
          (set `self.StolenRune` _returnvalue_2)
          (`self.K2_AttachToActor` _returnvalue_2 self "ForRune" "KeepWorld" "SnapToTarget" "KeepWorld" true)
          (`self.SetActorEnableCollision` _returnvalue_2 false)
          (`Widget.RemoveFromParent` _output))))))

(event `Mooving`
  (`SkeletalMeshComponent.PlayAnimation` (`self.Mesh`) "/Game/Mobs/Krab/A_KrabMooving.A_KrabMooving" (and (> (`self.Health`) 0.0) (<= (`KismetMathLibrary.Vector_Distance` (`self.K2_GetActorLocation` (`self.FPC`)) (`self.K2_GetActorLocation`)) 5000.0) (not (`self.HaveRune`))))
  (`GameplayStatics.SpawnSoundAttached` "/Game/Sounds/Sound_Krab_Cue.Sound_Krab_Cue" (`self.Sphere`) "None" (0.0 0.0 0.0) (struct) "KeepRelativeOffset" true 1.0 1.0 0.0 null null))

(event `WithRune`
  (`SkeletalMeshComponent.PlayAnimation` (`self.Mesh`) "/Game/Mobs/Krab/A_KrabArms.A_KrabArms" true))

(event `self.ReceiveTick`
  (params (DeltaSeconds :type "Float (single-precision)"))
  (bind _returnvalue (* 300 DeltaSeconds))
  (bind (_returnvalue_x _returnvalue_y) (`KismetMathLibrary.BreakVector` (`self.GetActorForwardVector` (`self.FPC`))))
  (if (<= (`KismetMathLibrary.Vector_Distance` (`self.K2_GetActorLocation` (`self.FPC`)) (`self.K2_GetActorLocation`)) 5000.0)
    (if (`self.HaveRune`)
      (`self.K2_AddActorLocalOffset` (`KismetMathLibrary.MakeVector` (* _returnvalue_x _returnvalue) (* _returnvalue_y _returnvalue)))
      (`/Engine/EditorBlueprintResources/StandardMacros.DoOnce` false
        (:`Completed`
          (`self.WithRune`)))
      (else
        (`AIBlueprintHelperLibrary.SimpleMoveToActor` (`AIBlueprintHelperLibrary.GetAIController` self) (`self.FPC`))
        (`/Engine/EditorBlueprintResources/StandardMacros.DoOnce` false :!label _label
          (:`Completed`
            (`self.Mooving`)))))
    (else
      (goto _label :!via `Reset`))))

(event `self.ReceiveBeginPlay`
  (bind (_textures_bombdamage _textures_bombgravity _textures_bombradius _textures_energy _textures_gunspeed _textures_shielddamage _textures_shieldregen) (break `/Game/System/RunesTextures` (`self.Textures`)))
  (bind _returnvalue (`GameplayStatics.GetActorOfClass` "/Game/FirstPersonBP/FirstPersonCharacter.FirstPersonCharacter_C"))
  (set `self.FPC` _returnvalue)
  (bind _returnvalue_2 (`PrimitiveComponent.CreateDynamicMaterialInstance` (`self.Plane`) 0 "/Game/Materials/M_Bullets2_Inst.M_Bullets2_Inst" "None"))
  (set `self.MI` _returnvalue_2)
  (bind _output_get (set `self.RuneInt` (`KismetMathLibrary.RandomIntegerInRange` 0 6)))
  (`MaterialInstanceDynamic.SetTextureParameterValue` (`self.MI`) "1" (select `int` _output_get :`0` _textures_bombdamage :`1` _textures_bombgravity :`2` _textures_bombradius :`3` _textures_energy :`4` _textures_gunspeed :`5` _textures_shielddamage :`6` _textures_shieldregen))
  (`MaterialInstanceDynamic.SetScalarParameterValue` (`self.MI`) "Emissive" 3.0)
  (`MaterialInstanceDynamic.SetVectorParameterValue` (`self.MI`) "Color" (make `LinearColor` 1.0 0.0 0.0 1.0)))

(event `LoosingHealth`
  (bind (_returnvalue_x _returnvalue_y _returnvalue_z) (`KismetMathLibrary.BreakVector` (`self.K2_GetActorLocation`)))
  (bind _stolenrune (`self.StolenRune`))
  (`MaterialInstanceDynamic.SetVectorParameterValue` (`self.MI`) "Color" (make `LinearColor` 1.0 (- 1.0 (/ (`self.Health`) (`self.MaxHealth`))) 0.0 1.0))
  (`GameplayStatics.PlaySoundAtLocation` "/Game/Sounds/Sound_Hit1.Sound_Hit1" (`self.K2_GetActorLocation` (`self.FPC`)) (struct) 1.0 1.0 0.0 null null null)
  (if (<= (`self.Health`) 0.0)
    (`/Engine/EditorBlueprintResources/StandardMacros.DoOnce` false
      (:`Completed`
        (`GameplayStatics.PlaySoundAtLocation` "/Game/Sounds/Sound_Death.Sound_Death" (`self.K2_GetActorLocation`) (struct) 1.0 1.0 0.0 null null null)
        (`SkeletalMeshComponent.PlayAnimation` (`self.Mesh`) "/Game/Mobs/Krab/A_KrabDeath.A_KrabDeath" false)
        (`KismetSystemLibrary.Delay` 1.0)
        (`|SpawnActorFromClass` (select `int` (`self.RuneInt`) :`0` "/Game/Runes/Loot/Damage.Damage_C" :`1` "/Game/Runes/Loot/Gravity.Gravity_C" :`2` "/Game/Runes/Loot/Radius.Radius_C" :`3` "/Game/Runes/Loot/Energy.Energy_C" :`4` "/Game/Runes/Loot/Speed.Speed_C" :`5` "/Game/Runes/Loot/ShieldDamage.ShieldDamage_C" :`6` "/Game/Runes/Loot/ShieldRegen.ShieldRegen_C" :!type "Actor Class Reference") (`KismetMathLibrary.MakeTransform` (`KismetMathLibrary.MakeVector` _returnvalue_x _returnvalue_y (+ _returnvalue_z 100.0)) (struct) (`SceneComponent.K2_GetComponentScale` (`self.Plane`))) "Undefined" "OverrideRootScale" null null)
        (`/Engine/EditorBlueprintResources/StandardMacros.IsValid` _stolenrune
          (:`Is Valid`
            (`self.K2_DetachFromActor` _stolenrune "KeepWorld" "KeepWorld" "KeepRelative")
            (`self.SetActorEnableCollision` _stolenrune true))
          (:`Is Not Valid`
            _))
        (`|SpawnActorFromClass` "/Game/Mobs/BP_Mask.BP_Mask_C" (`KismetMathLibrary.MakeTransform` (`self.K2_GetActorLocation`)) "Undefined" "OverrideRootScale" null null)
        (`self.K2_DestroyActor`)))))

(event `self.ReceiveAnyDamage`
  (params (Damage :type "Float (single-precision)") (DamageType :type "DamageType Object Reference") (InstigatedBy :type "Controller Object Reference") (DamageCauser :type "Actor Object Reference"))
  (set `self.Health` (- (`self.Health`) Damage))
  (`self.LoosingHealth`))

(event `self.Box2.OnComponentBeginOverlap`
  (params (OverlappedComponent :type "PrimitiveComponent Object Reference") (OtherActor :type "Actor Object Reference") (OtherComp :type "PrimitiveComponent Object Reference") (OtherBodyIndex :type Integer) (bFromSweep :type Boolean) (SweepResult :type "HitResult Structure (by ref)"))
  (bind _gun1_damage (break `/Game/System/BPS_Gun1` (`/Game/FirstPersonBP/FirstPersonCharacter.Gun1` (`self.FPC`))))
  (cast `/Game/FirstPersonBP/BP_Bomb2` OtherActor
    (:`then`
      _)
    (:`CastFailed`
      (cast `/Game/FirstPersonBP/BP_Bullet` OtherActor)))
  (set `self.Health` (- (`self.Health`) (* 2 _gun1_damage)))
  (`self.LoosingHealth`))

(event `self.Box3.OnComponentBeginOverlap`
  (params (OverlappedComponent :type "PrimitiveComponent Object Reference") (OtherActor :type "Actor Object Reference") (OtherComp :type "PrimitiveComponent Object Reference") (OtherBodyIndex :type Integer) (bFromSweep :type Boolean) (SweepResult :type "HitResult Structure (by ref)"))
  (bind _gun1_damage (break `/Game/System/BPS_Gun1` (`/Game/FirstPersonBP/FirstPersonCharacter.Gun1` (`self.FPC`))))
  (cast `/Game/FirstPersonBP/BP_Bomb2` OtherActor
    (:`then`
      _)
    (:`CastFailed`
      (cast `/Game/FirstPersonBP/BP_Bullet` OtherActor)))
  (set `self.Health` (- (`self.Health`) (* 2 _gun1_damage)))
  (`self.LoosingHealth`))

(fn `UserConstructionScript`)