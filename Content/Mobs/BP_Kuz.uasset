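; BP_Kuz is a mob character that hops on the spot by repeatedly playing a jump montage at increased speed.
; BeginPlay plays it once and starts a looping one-second timer that replays it.
; Montage notify begin and end drive Jump and StopJumping, syncing the hop to the animation.
; It caches the FirstPersonCharacter, but the logic to face and move ahead of that player is disconnected and never runs.
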(event `self.ReceiveTick`
  (params (DeltaSeconds :type "Float (single-precision)")))

(event `self.ReceiveBeginPlay`
  (bind _returnvalue (`GameplayStatics.GetActorOfClass` "/Game/FirstPersonBP/FirstPersonCharacter.FirstPersonCharacter_C"))
  (set `self.FPC` _returnvalue)
  (`/Engine/EditorBlueprintResources/StandardMacros.DoOnce` false
    (:`Completed`
      (`|PlayMontage` (`self.Mesh`) "/Game/Mobs/K_Jump_Montage.K_Jump_Montage" 3.0
        (:`then`
          (`KismetSystemLibrary.K2_SetTimerDelegate` (delegate `CustomEvent_0`) 1.0 true))
        (:`OnNotifyBegin`
          (`self.Jump`))
        (:`OnNotifyEnd`
          (`self.StopJumping`))))))

(event `CustomEvent_0`
  (`|PlayMontage` (`self.Mesh`) "/Game/Mobs/K_Jump_Montage.K_Jump_Montage" 3.0
    (:`OnNotifyBegin`
      (`self.Jump`))
    (:`OnNotifyEnd`
      (`self.StopJumping`))))

(fn `UserConstructionScript`)