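; Grasshopper (Kuznechik) enemy that damages the player on overlap and drops a random rune pickup plus BP_Mask on death.
; Player proximity starts a looping timer replaying the jump montage, whose notifies toggle Mooving and walk speed.
; A socketed plane's dynamic material shows the rune and shifts red to yellow as health falls.
; Socketed box takes double gun damage from bullets and bombs; chase and facing code is disconnected.
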(event `self.ReceiveTick`
  (params (DeltaSeconds :type "Float (single-precision)"))
  (if (<= (`self.GetDistanceTo` (`self.FPC`) self) 5000.0)
    (`/Engine/EditorBlueprintResources/StandardMacros.DoOnce` false :!label _label
      (:`Completed`
        (`self.NearTrue`)))
    (else
      (`KismetSystemLibrary.K2_ClearAndInvalidateTimerHandle` (stale `NearTrue` _returnvalue))
      (goto _label :!via `Reset`))))

(event `self.ReceiveActorBeginOverlap`
  (params (OtherActor :type "Actor Object Reference"))
  (bind _asfirst_person_character (cast `/Game/FirstPersonBP/FirstPersonCharacter` OtherActor))
  (set `self.Attacked` true)
  (`GameplayStatics.ApplyDamage` _asfirst_person_character 15.0)
  (`KismetSystemLibrary.Delay` 2.0)
  (set `self.Attacked` false))

(event `NearTrue`
  (`|PlayMontage` (`self.Mesh`) "/Game/Mobs/Kuznechik/Test2/K_JLM.K_JLM"
    (:`then`
      (bind _returnvalue (`KismetSystemLibrary.K2_SetTimerDelegate` (delegate `CustomEvent_0`) 1.0 true)))
    (:`OnNotifyBegin`
      (set `self.Mooving` true))
    (:`OnNotifyEnd`
      (set `self.Mooving` false)
      (`GameplayStatics.PlaySoundAtLocation` "/Game/Sounds/Sound_KuzJump_Cue.Sound_KuzJump_Cue" (`self.K2_GetActorLocation`) (struct) 1.0 1.0 0.0 null null null))))

(event `self.ReceiveBeginPlay`
  (bind (_textures_bombdamage _textures_bombgravity _textures_bombradius _textures_energy _textures_gunspeed _textures_shielddamage _textures_shieldregen) (break `/Game/System/RunesTextures` (`self.Textures`)))
  (`SceneComponent.K2_AttachToComponent` (`self.Box`) (`self.Mesh`) "BoxSocket" "SnapToTarget" "SnapToTarget" "KeepWorld" true)
  (`SceneComponent.K2_AttachToComponent` (`self.Plane`) (`self.Mesh`) "RuneSocket" "SnapToTarget" "SnapToTarget" "KeepWorld" true)
  (bind _returnvalue (`PrimitiveComponent.CreateDynamicMaterialInstance` (`self.Plane`) 0 "/Game/Materials/M_Bullets2_Inst.M_Bullets2_Inst" "None"))
  (set `self.MI` _returnvalue)
  (bind _output_get (set `self.RuneInt` (`KismetMathLibrary.RandomIntegerInRange` 0 6)))
  (`MaterialInstanceDynamic.SetTextureParameterValue` (`self.MI`) "1" (select `int` _output_get :`0` _textures_bombdamage :`1` _textures_bombgravity :`2` _textures_bombradius :`3` _textures_energy :`4` _textures_gunspeed :`5` _textures_shielddamage :`6` _textures_shieldregen))
  (`MaterialInstanceDynamic.SetScalarParameterValue` (`self.MI`) "Emissive" 3.0)
  (`MaterialInstanceDynamic.SetVectorParameterValue` (`self.MI`) "Color" (make `LinearColor` 1.0 0.0 0.0 1.0))
  (bind _returnvalue_2 (`GameplayStatics.GetActorOfClass` "/Game/FirstPersonBP/FirstPersonCharacter.FirstPersonCharacter_C"))
  (set `self.FPC` _returnvalue_2))

(event `CustomEvent_0`
  (bind _notifyname (`|PlayMontage` (`self.Mesh`) "/Game/Mobs/Kuznechik/Test2/K_JLM.K_JLM")
    (:`OnNotifyBegin`
      (if (== _notifyname "Middle")
        (set `CharacterMovementComponent.MaxWalkSpeed` 1000.0 (`self.CharacterMovement`))
        (else
          (set `self.Mooving` true))))
    (:`OnNotifyEnd`
      (set `self.Mooving` false)
      (set `CharacterMovementComponent.MaxWalkSpeed` 6000.0 (`self.CharacterMovement`))
      (`GameplayStatics.PlaySoundAtLocation` "/Game/Sounds/Sound_KuzJump_Cue.Sound_KuzJump_Cue" (`self.K2_GetActorLocation`) (struct) 1.0 1.0 0.0 null null null))))

(event `LoosingHealth`
  (bind (_returnvalue_x _returnvalue_y _returnvalue_z) (`KismetMathLibrary.BreakVector` (`self.K2_GetActorLocation`)))
  (`MaterialInstanceDynamic.SetVectorParameterValue` (`self.MI`) "Color" (make `LinearColor` 1.0 (- 1.0 (/ (`self.Health`) (`self.MaxHealth`))) 0.0 1.0))
  (`GameplayStatics.PlaySoundAtLocation` "/Game/Sounds/Sound_Hit1.Sound_Hit1" (`self.K2_GetActorLocation` (`self.FPC`)) (struct) 1.0 1.0 0.0 null null null)
  (if (<= (`self.Health`) 0.0)
    (`/Engine/EditorBlueprintResources/StandardMacros.DoOnce` false
      (:`Completed`
        (`KismetSystemLibrary.K2_ClearAndInvalidateTimerHandle` (stale `NearTrue` _returnvalue))
        (set `self.Mooving` false)
        (`GameplayStatics.PlaySoundAtLocation` "/Game/Sounds/Sound_Death.Sound_Death" (`self.K2_GetActorLocation`) (struct) 1.0 1.0 0.0 null null null)
        (`SkeletalMeshComponent.PlayAnimation` (`self.Mesh`) "/Game/Mobs/Kuznechik/Test2/KuzDeath.KuzDeath" false)
        (`KismetSystemLibrary.Delay` 1.0)
        (`|SpawnActorFromClass` (select `int` (`self.RuneInt`) :`0` "/Game/Runes/Loot/Damage.Damage_C" :`1` "/Game/Runes/Loot/Gravity.Gravity_C" :`2` "/Game/Runes/Loot/Radius.Radius_C" :`3` "/Game/Runes/Loot/Energy.Energy_C" :`4` "/Game/Runes/Loot/Speed.Speed_C" :`5` "/Game/Runes/Loot/ShieldDamage.ShieldDamage_C" :`6` "/Game/Runes/Loot/ShieldRegen.ShieldRegen_C" :!type "Actor Class Reference") (`KismetMathLibrary.MakeTransform` (`KismetMathLibrary.MakeVector` _returnvalue_x _returnvalue_y (+ _returnvalue_z 100.0)) (struct) (`SceneComponent.K2_GetComponentScale` (`self.Plane`))) "Undefined" "OverrideRootScale" null null)
        (`|SpawnActorFromClass` "/Game/Mobs/BP_Mask.BP_Mask_C" (`KismetMathLibrary.MakeTransform` (`self.K2_GetActorLocation`)) "Undefined" "OverrideRootScale" null null)
        (`self.K2_DestroyActor`)))))

(event `self.ReceiveAnyDamage`
  (params (Damage :type "Float (single-precision)") (DamageType :type "DamageType Object Reference") (InstigatedBy :type "Controller Object Reference") (DamageCauser :type "Actor Object Reference"))
  (set `self.Health` (- (`self.Health`) Damage))
  (`self.LoosingHealth`))

(event `self.Box.OnComponentBeginOverlap`
  (params (OverlappedComponent :type "PrimitiveComponent Object Reference") (OtherActor :type "Actor Object Reference") (OtherComp :type "PrimitiveComponent Object Reference") (OtherBodyIndex :type Integer) (bFromSweep :type Boolean) (SweepResult :type "HitResult Structure (by ref)"))
  (bind _gun1_damage (break `/Game/System/BPS_Gun1` (`/Game/FirstPersonBP/FirstPersonCharacter.Gun1` (`self.FPC`))))
  (cast `/Game/FirstPersonBP/BP_Bomb2` OtherActor
    (:`then`
      _)
    (:`CastFailed`
      (cast `/Game/FirstPersonBP/BP_Bullet` OtherActor)))
  (set `self.Health` (- (`self.Health`) (* 2 _gun1_damage)))
  (`self.LoosingHealth`))

(fn `UserConstructionScript`)