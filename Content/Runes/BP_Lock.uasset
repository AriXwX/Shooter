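; BP_Lock is a rune lock that displays two textures on glowing planes and triggers a door when the player's runes match.
; On damage or overlap with a bullet or bomb, it gathers image textures from the player's active-slot widget and compares their names to its own.
; At two or more matches, Task selects which door Blueprint to trigger, falling or placing, and the lock destroys itself.
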(event `self.ReceiveBeginPlay`
  (bind _returnvalue (`GameplayStatics.GetActorOfClass` "/Game/FirstPersonBP/FirstPersonCharacter.FirstPersonCharacter_C"))
  (bind _returnvalue_2 (`PrimitiveComponent.CreateDynamicMaterialInstance` (`self.Plane`) 0 "/Game/Materials/M_Bullets2_Inst.M_Bullets2_Inst" "None"))
  (`MaterialInstanceDynamic.SetTextureParameterValue` _returnvalue_2 "1" (`self.Texture1`))
  (`MaterialInstanceDynamic.SetScalarParameterValue` _returnvalue_2 "Emissive" 5.0)
  (bind _returnvalue_3 (`PrimitiveComponent.CreateDynamicMaterialInstance` (`self.Plane1`) 0 "/Game/Materials/M_Bullets2_Inst.M_Bullets2_Inst" "None"))
  (`MaterialInstanceDynamic.SetTextureParameterValue` _returnvalue_3 "1" (`self.Texture2`))
  (`MaterialInstanceDynamic.SetScalarParameterValue` _returnvalue_3 "Emissive" 10.0))

(event `self.ReceiveAnyDamage`
  (params (Damage :type "Float (single-precision)") (DamageType :type "DamageType Object Reference") (InstigatedBy :type "Controller Object Reference") (DamageCauser :type "Actor Object Reference"))
  (bind _wbpas (`/Game/FirstPersonBP/FirstPersonCharacter.WBPAS` (stale `self.ReceiveBeginPlay` _returnvalue)))
  (for _array_element (`PanelWidget.GetAllChildren` (select `int` (`/Game/FirstPersonBP/FirstPersonCharacter.ActiveSlotNumber` (stale `self.ReceiveBeginPlay` _returnvalue)) :`0` (`/Game/Runes/ActiveSlots/WBP_ActiveSlot1.Overlay_112` (`/Game/Runes/ActiveSlots/WBP_ActiveSlots.WBP_ActiveSlot1` _wbpas)) :`1` (`/Game/Runes/ActiveSlots/WBP_ActiveSlot2.Overlay_112` (`/Game/Runes/ActiveSlots/WBP_ActiveSlots.WBP_ActiveSlot2` _wbpas)) :`2` (`/Game/Runes/ActiveSlots/WBP_ActiveSlot3.Overlay_112` (`/Game/Runes/ActiveSlots/WBP_ActiveSlots.WBP_ActiveSlot3` _wbpas)))) :!label _label
    (bind _aswbp_slot_2 (cast `/Game/Runes/WBP_Slot2` _array_element))
    (bind (_brush_imagesize _brush_margin _brush_tintcolor _brush_resourceobject) (break `SlateBrush` (`Image.Brush` (`/Game/Runes/WBP_Slot2.Image` _aswbp_slot_2))))
    (bind _astexture (cast `Texture` _brush_resourceobject))
    (`KismetArrayLibrary.Array_AddUnique` (`self.As Texture`) _astexture))
  (for _array_element_2 (`self.As Texture`)
    (bind _returnvalue (`KismetSystemLibrary.GetObjectName` _array_element_2))
    (if (or (`KismetStringLibrary.EqualEqual_StrStr` _returnvalue (`KismetSystemLibrary.GetObjectName` (`self.Texture1`))) (`KismetStringLibrary.EqualEqual_StrStr` _returnvalue (`KismetSystemLibrary.GetObjectName` (`self.Texture2`))))
      (`/Engine/EditorBlueprintResources/StandardMacros.IncrementInt` (`self.Done`))))
  (if (>= (`self.Done`) 2)
    (switch `int` (`self.Task`)
      (:`0`
        (bind _returnvalue_2 (`GameplayStatics.GetActorOfClass` "/Game/Runes/Up_Door_Blueprint.Up_Door_Blueprint_C"))
        (`/Game/Runes/Up_Door_Blueprint.Falling` _returnvalue_2))
      (:`1`
        (bind _returnvalue_3 (`GameplayStatics.GetActorOfClass` "/Game/Sounds/Right_Door9_Blueprint.Right_Door9_Blueprint_C"))
        (`/Game/Sounds/Right_Door9_Blueprint.Placing` _returnvalue_3)))
    (`self.K2_DestroyActor`)
    (else
      (set `self.Done` 0))))

(event `self.ReceiveActorBeginOverlap`
  (params (OtherActor :type "Actor Object Reference"))
  (cast `/Game/FirstPersonBP/BP_Bullet` OtherActor
    (:`then`
      (goto _label))
    (:`CastFailed`
      (cast `/Game/FirstPersonBP/BP_Bomb2` OtherActor)
      (goto _label))))

(fn `UserConstructionScript`)