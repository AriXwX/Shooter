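; A rune Blueprint that adds a damage rune to the player's screen when the first-person character overlaps it.
; Each overlap creates a WBP_RunesParent widget, stores it in the character's RunesOnScreen3 array and plays its animation.
; The widget takes its texture and damage value, stored as Gun, from the character's RuneDamage data.
; After a short delay, it calls the character's BackPack function if the array's first widget is valid.
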(event `self.ReceiveActorBeginOverlap`
  (params (OtherActor :type "Actor Object Reference"))
  (bind _asfirst_person_character (cast `/Game/FirstPersonBP/FirstPersonCharacter` OtherActor))
  (bind _returnvalue (`|CreateWidget` "/Game/Runes/WBP_RunesParent.WBP_RunesParent_C"))
  (`UserWidget.AddToViewport` _returnvalue 0)
  (bind _runesonscreen3 (`/Game/FirstPersonBP/FirstPersonCharacter.RunesOnScreen3` _asfirst_person_character))
  (bind _returnvalue_2 (`KismetArrayLibrary.Array_Add` _runesonscreen3 _returnvalue))
  (bind _output (`|GetArrayItem` _runesonscreen3 _returnvalue_2))
  (`Widget.SetVisibility` _output "Visible")
  (bind _runedamage (`/Game/FirstPersonBP/FirstPersonCharacter.RuneDamage` _asfirst_person_character))
  (bind _texture (`/Game/Runes/WBPRunes/WBP_Damage.Texture` _runedamage))
  (`Image.SetBrushFromTexture` (`/Game/Runes/WBP_RunesParent.Image` _output) _texture false)
  (bind _output_2 (`|GetArrayItem` _runesonscreen3 _returnvalue_2))
  (`UserWidget.PlayAnimation` _output_2 (`/Game/Runes/WBP_RunesParent.NewAnimation` _output_2) 0.0 1 "Forward" 1.0 false)
  (bind _output_3 (`|GetArrayItem` _runesonscreen3 _returnvalue_2))
  (set `/Game/Runes/WBP_RunesParent.Texture` _texture _output_3)
  (set `/Game/Runes/WBP_RunesParent.Gun` (`/Game/Runes/WBPRunes/WBP_Damage.Damage` _runedamage) _output_3)
  (`KismetSystemLibrary.Delay` 2.0)
  (if (`KismetSystemLibrary.IsValid` (`|GetArrayItem` _runesonscreen3))
    (`/Game/FirstPersonBP/FirstPersonCharacter.BackPack` _asfirst_person_character)))

(fn `UserConstructionScript`)